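; ConditionalDoor_BP is an interactable locked door that opens when the player carries its matching key item.
; On BeginPlay it caches the required name from the KeyInStage reference.
; On interaction it searches the third-person character's KeyItemRing by name, printing "Locked!" for each non-match checked.
; A found key destroys the Cube2 component to clear the door and is removed from the ring.
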(event `self.ReceiveBeginPlay`
  (`parent.ReceiveBeginPlay`)
  (bind _output_get (set `self.KeySavedLocal` (`self.KeyInStage`)))
  (bind _keyiteminfo_name (break `/Game/Bunker/KeyItem_Struct` (`/Game/Bunker/KeyItemPickup_BP.KeyItemInfo` _output_get)))
  (set `self.Required Key Name` _keyiteminfo_name))

(event `/Game/Bunker/Interaction_BPI.InteractWithActor`
  (`parent.InteractWithActor`)
  (bind _asbp_third_person_character (cast `/Game/ThirdPerson/Blueprints/BP_ThirdPersonCharacter` (`GameplayStatics.GetPlayerCharacter` 0)))
  (bind _keyitemring (`/Game/ThirdPerson/Blueprints/BP_ThirdPersonCharacter.KeyItemRing` _asbp_third_person_character))
  (for _array_element _keyitemring
    (bind _keyitemdata_name (break `/Game/Bunker/KeyItem_Struct` (`/Game/Bunker/KeyItem_UBP.KeyItemData` _array_element)))
    (if (== _keyitemdata_name (`self.Required Key Name`))
      (set `self.Required Key` _array_element)
      (break)
      (else
        (`KismetSystemLibrary.PrintString` "Locked!" true true (struct :`R` 1.0 :`G` 0.174958 :`B` 0.182916 :`A` 1.0)))))
  (for _array_element_2 _keyitemring
    (if (== _array_element_2 (`self.Required Key`))
      (`ActorComponent.K2_DestroyComponent` (`self.Cube2`))
      (break)))
  (`KismetArrayLibrary.Array_RemoveItem` _keyitemring (`self.Required Key`)))

(fn `UserConstructionScript`
  (`parent.UserConstructionScript`))